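; Database connector that handles account login and registration against a SQL users table for the W_LoadGame menu.
; A UMG_DBConnection widget supplies connection details, while login and register checks run selects built by raw string concatenation, including unhashed passwords.
; The Operation variable routes results: login saves name and rank to the "user" save slot, registration inserts untaken accounts.
; Outcomes are pushed to every W_LoadGame widget found.
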(event Custom|Login
  (params (Server :type String) (DBName :type String) (User%20ID :type String) (Password :type String) (Extra%20Params :type Map%20of%20Strings%20to%20Strings))
  (Class|MySQLDBConnectionActor|CreateNewConnection Server DBName User%20ID Password Extra%20Params))

(event Custom|RegisterCheck
  (params (Name :type String) (Email :type String) (Password :type String))
  (Variables|Default|Setoperation "Register")
  (Class|MySQLDBConnectionActor|SelectDatafromQuery 0 (Utilities|String|Append "select * from users where name = " "\"" Name "\"" " or " "email = " "\"" Email "\"")))

(event Custom|SearchUser
  (params (Name :type String) (Password :type String))
  (Variables|Default|Setoperation "Login")
  (Class|MySQLDBConnectionActor|SelectDatafromQuery 0 (Utilities|String|Append "select * from users where name = " "\"" Name "\"" " and " "password = " "\"" Password "\"")))

(event EventBeginPlay
  (|CallParentFunction)
  (bind _returnvalue (UserInterface|CreateWidget "/MySQL/Widgets/UMG_DBConnection.UMG_DBConnection_C"))
  (UserInterface|Viewport|AddtoViewport _returnvalue 0)
  (EventDispatchers|BindEventtoOnLoggingin _returnvalue (delegate Custom|Login)))

(event EventOnCallUpdateQuery
  (params (UpdateQuery :type String) (QueryID :type Integer))
  (Class|MySQLDBConnectionActor|UpdateDatafromQuery 0 UpdateQuery))

(event EventOnQueryUpdateStatusChanged
  (params (IsSuccessful :type Boolean) (ErrorMessage :type String))
  (if IsSuccessful
    (bind _foundwidgets (Widget|GetAllWidgetsOfClass "/Game/Blueprints/Widgets/W_LoadGame.W_LoadGame_C" true))
    (for _array_element _foundwidgets
      (Rendering|Components|TextRender|SetText (Variables|/Game/Blueprints/Widgets/W_LoadGame.W_LoadGame_C|Geterror_1 _array_element) "Account Succesfully Created.")
      (Appearance|SetColorandOpacity (Variables|/Game/Blueprints/Widgets/W_LoadGame.W_LoadGame_C|Geterror_1 _array_element) (Utilities|Struct|MakeSlateColor "(R=0.024414,G=1.000000,B=0.000000,A=1.000000)" "UseColor_Specified") :!class /Script/UMG.TextBlock))
    (else
      (Development|PrintString ErrorMessage)
      (bind _foundwidgets_2 (Widget|GetAllWidgetsOfClass "/Game/Blueprints/Widgets/W_LoadGame.W_LoadGame_C" true))
      (for _array_element_2 _foundwidgets_2
        (Rendering|Components|TextRender|SetText (Variables|/Game/Blueprints/Widgets/W_LoadGame.W_LoadGame_C|Geterror_1 _array_element_2) "Account Fail Created.")
        (Appearance|SetColorandOpacity (Variables|/Game/Blueprints/Widgets/W_LoadGame.W_LoadGame_C|Geterror_1 _array_element_2) (Utilities|Struct|MakeSlateColor "(R=1.000000,G=0.000000,B=0.023529,A=1.000000)" "UseColor_Specified") :!class /Script/UMG.TextBlock)))))

(event EventOnConnectionStateChanged
  (params (ConnectionStatus :type Boolean) (ConnectionID :type Integer) (ErrorMessage :type String))
  (Default|OnConnectionChanged (stale EventBeginPlay _returnvalue) ConnectionStatus ErrorMessage))

(event EventOnQuerySelectStatusChanged
  (params (IsSuccessful :type Boolean) (ErrorMessage :type String) (ResultByColumn :type Array%20of%20My%20SQL%20Data%20Table%20Structures) (ResultByRow :type Array%20of%20My%20SQL%20Data%20Row%20Structures))
  (bind _operation (Variables|Default|Getoperation))
  (if (Utilities|Enum|Equal(Enum) _operation "Login")
    (Variables|Default|SetHave? false)
    (if IsSuccessful
      (Utilities|FlowControl|Sequence
        (:then_0
          (for _array_element ResultByRow
            (for _array_element_2 (Utilities|Struct|BreakMySQLDataRow _array_element)
              (Utilities|FlowControl|DoOnce false
                (:Completed
                  (if (Utilities|Enum|NotEqual(Enum) _array_element_2 "")
                    (Variables|Default|SetHave? true)
                    (bind _output_get (Variables|Default|SetUserInfo (Utilities|Struct|BreakMySQLDataRow _array_element)))))))
            (Utilities|FlowControl|Sequence
              (:then_0
                (Utilities|FlowControl|DoOnce false) ; enters at Reset
              )
              (:then_1
                (if (not (Variables|Default|GetHave?))
                  (bind _foundwidgets (Widget|GetAllWidgetsOfClass "/Game/Blueprints/Widgets/W_LoadGame.W_LoadGame_C" true))
                  (for _array_element_3 _foundwidgets
                    (Rendering|Components|TextRender|SetText (Variables|/Game/Blueprints/Widgets/W_LoadGame.W_LoadGame_C|Geterror _array_element_3) "Failed Login. Username or Password dont exist.")
                    (Appearance|SetColorandOpacity (Variables|/Game/Blueprints/Widgets/W_LoadGame.W_LoadGame_C|Geterror _array_element_3) (Utilities|Struct|MakeSlateColor "(R=1.000000,G=0.000000,B=0.024480,A=1.000000)" "UseColor_Specified") :!class /Script/UMG.TextBlock))))
              (:then_2
                (if (Variables|Default|GetHave?)
                  (bind _returnvalue (SaveGame|LoadGamefromSlot "user"))
                  (bind _asbp_user_save_game (Utilities|Casting|CastToBP_UserSaveGame _returnvalue))
                  (Variables|/Script/Ghostcore.UserSaveGame|SetPlayerName _asbp_user_save_game (Utilities|Array|Get(acopy) _output_get 1))
                  (Variables|/Script/Ghostcore.UserSaveGame|SetRank _asbp_user_save_game (Utilities|Array|Get(acopy) _output_get 4))
                  (bind _returnvalue_2 (SaveGame|SaveGametoSlot _asbp_user_save_game "user"))
                  (if _returnvalue_2
                    (bind _foundwidgets_2 (Widget|GetAllWidgetsOfClass "/Game/Blueprints/Widgets/W_LoadGame.W_LoadGame_C" true))
                    (for _array_element_4 _foundwidgets_2
                      (Default|SuccessLogin _array_element_4)
                      (Class|MySQLDBConnectionActor|CloseConnection))
                    (else
                      (bind _foundwidgets_3 (Widget|GetAllWidgetsOfClass "/Game/Blueprints/Widgets/W_LoadGame.W_LoadGame_C" true))
                      (for _array_element_5 _foundwidgets_3
                        (Rendering|Components|TextRender|SetText (Variables|/Game/Blueprints/Widgets/W_LoadGame.W_LoadGame_C|Geterror _array_element_5) "Failed Login. Try again later.")
                        (Appearance|SetColorandOpacity (Variables|/Game/Blueprints/Widgets/W_LoadGame.W_LoadGame_C|Geterror _array_element_5) (Utilities|Struct|MakeSlateColor "(R=1.000000,G=0.000000,B=0.024480,A=1.000000)" "UseColor_Specified") :!class /Script/UMG.TextBlock)))))))))))
    (else
      (Variables|Default|SetHave? false)
      (if (Utilities|Enum|Equal(Enum) _operation "Register")
        (for _array_element_6 ResultByRow
          (for _array_element_7 (Utilities|Struct|BreakMySQLDataRow _array_element_6)
            (Utilities|FlowControl|DoOnce false
              (:Completed
                (if (Utilities|Enum|NotEqual(Enum) _array_element_7 "")
                  (Variables|Default|SetHave? true)))))
          (Utilities|FlowControl|Sequence
            (:then_0
              (Utilities|FlowControl|DoOnce false) ; enters at Reset
            )
            (:then_1
              (if (Variables|Default|GetHave?)
                (bind _foundwidgets_4 (Widget|GetAllWidgetsOfClass "/Game/Blueprints/Widgets/W_LoadGame.W_LoadGame_C" true))
                (for _array_element_8 _foundwidgets_4
                  (Rendering|Components|TextRender|SetText (Variables|/Game/Blueprints/Widgets/W_LoadGame.W_LoadGame_C|Geterror _array_element_8) "Failed Create Account. Username or Email is already taken.")
                  (Appearance|SetColorandOpacity (Variables|/Game/Blueprints/Widgets/W_LoadGame.W_LoadGame_C|Geterror _array_element_8) (Utilities|Struct|MakeSlateColor "(R=1.000000,G=0.000000,B=0.023529,A=1.000000)" "UseColor_Specified") :!class /Script/UMG.TextBlock))
                (else
                  (Development|PrintString "asdasd")
                  (CallFunction|OnCallUpdateQuery (Utilities|String|Append "INSERT INTO users (`name`, `email`, `password`, `rank`, `timestmap`) VALUES" " (\"" (stale Custom|RegisterCheck Name) "\",\"" (stale Custom|RegisterCheck Email) "\",\"" (stale Custom|RegisterCheck Password) "\",\"GHOST HUNTIN' INVESTIGATOR\", current_timestamp())")))))))))))

(fn ConstructionScript
  (|CallParentFunction))

(fn ReturnUserData
  (params (Name :type String) (Password :type String))
  (Class|MySQLDBConnectionActor|SelectDatafromQuery 0 (Utilities|String|Append "select * from users where name == " Name)))